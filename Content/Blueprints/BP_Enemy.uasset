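; BP_Enemy is a turret-style enemy that aims at the player character and fires projectiles at a fixed interval.
; BeginPlay caches the AsdfCharacter found in the level, keeping the last one if several exist.
; Each Tick turns Weaponbase toward the character's capsule by adding a relative look-at rotation, with no interpolation or range check.
; A countdown reset to Timetoshoot spawns BP_ProjectileActor at the Muzzle transform.
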(event `self.ReceiveBeginPlay`
  (set `self.time since shoot` (`self.timetoshoot`))
  (bind _outactors (`GameplayStatics.GetAllActorsOfClass` "/Script/asdfasdffinal.AsdfCharacter"))
  (for _array_element _outactors
    (set `self.character` _array_element)))

(event `self.ReceiveTick`
  (params (DeltaSeconds :type "Float (single-precision)"))
  (`self.tracking`)
  (bind _output_get (set `self.time since shoot` (- (`self.time since shoot`) DeltaSeconds)))
  (if (< _output_get 0.0)
    (set `self.time since shoot` (`self.timetoshoot`))
    (`self.shootnow`)))

(fn `shootnow`
  (`|SpawnActorFromClass` "/Game/Blueprints/BP_ProjectileActor.BP_ProjectileActor_C" (`SceneComponent.K2_GetComponentToWorld` (`self.muzzle`)) "Undefined" "MultiplyWithRoot" null null))

(fn `tracking`
  (bind _weaponbase (`self.weaponbase`))
  (`SceneComponent.K2_AddRelativeRotation` _weaponbase (`KismetMathLibrary.FindRelativeLookAtRotation` (`SceneComponent.K2_GetComponentToWorld` _weaponbase) (`SceneComponent.K2_GetComponentLocation` (`Character.CapsuleComponent` (`self.character`)))) false false))

(fn `UserConstructionScript`)